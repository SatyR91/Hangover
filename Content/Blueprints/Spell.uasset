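; Spell Blueprint that tracks whether a spell is unlocked and off cooldown.
; SpellInCooldown starts a looping one-second timer that calls DecreaseCooldown to count the Cooldown value down.
; Tick clears that timer through SpellNotInCooldown whenever the spell is unlocked and the cooldown has run out.
; IsCastable reports readiness and prints a debug message when the spell is locked or still cooling down.
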(event Custom|SpellInCooldown
  (bind _returnvalue (Utilities|Time|SetTimerbyFunctionName 0 "DecreaseCooldown" 1.0 true))
  (Development|PrintString (Utilities|String|ToString(Float) (Variables|Default|GetCooldown))))

(event Custom|SpellNotInCooldown
  (Utilities|Time|ClearandInvalidateTimerbyHandle (stale Custom|SpellInCooldown _returnvalue)))

(event EventBeginPlay)

(event EventTick
  (params (DeltaSeconds :type Float%20%28single-precision%29))
  (if (Variables|Default|GetUnlocked)
    (if (<= (Variables|Default|GetCooldown) 0.0)
      (CallFunction|SpellNotinCooldown))))

(fn IsCastable
  (bind _cooldown (Variables|Default|GetCooldown))
  (bind _unlocked (Variables|Default|GetUnlocked))
  (bind _returnvalue (<= _cooldown 0.0))
  (bind _returnvalue_2 (and _returnvalue _unlocked))
  (if _unlocked
    (if _returnvalue
      (return _returnvalue_2)
      (else
        (Development|PrintString "Spell is not ready")
        (return _returnvalue_2)))
    (else
      (Development|PrintString "Speel is not unlocked yet")
      (return _returnvalue_2))))

(fn DecreaseCooldown
  (Variables|Default|SetCooldown (- (Variables|Default|GetCooldown) 1.0)))